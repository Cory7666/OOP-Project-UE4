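; BP_BaseThing is a base Blueprint for damageable, destroyable items, with empty effect hooks.
; OnGetDamage subtracts damage while Health is above zero, logs the hit and calls Effect.
; OnDeath logs the killer, then calls EffectOnDeath and destroys the actor unless god mode is enabled.
; The damage event does not trigger death itself, and god mode does not block damage.
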(event `OnGetDamage`
  (params (DamageSize :type "Float (double-precision)") (DamagedBy :type "Actor Object Reference"))
  (bind _health (`self.Health`))
  (if (> _health 0.0)
    (bind _output_get (set `self.Health` (- _health DamageSize)))
    (`KismetSystemLibrary.PrintString` (`KismetStringLibrary.Concat_StrStr` "Got damage [" (`KismetStringLibrary.Conv_DoubleToString` DamageSize) "] from [" (`KismetSystemLibrary.GetDisplayName` DamagedBy) "]. Now health is " (`KismetStringLibrary.Conv_DoubleToString` _output_get) ".") false)
    (`self.Effect` DamagedBy)))

(event `OnDeath`
  (params (KilledBy :type "Actor Object Reference"))
  (if (`self.IsGodModEnabled`)
    (`KismetSystemLibrary.PrintString` (`KismetStringLibrary.Concat_StrStr` "[" (`KismetSystemLibrary.GetDisplayName` KilledBy) "] tried to kill [" (`KismetSystemLibrary.GetDisplayName` self) "], but can't: God mode enabled.") false)
    (else
      (`KismetSystemLibrary.PrintString` (`KismetStringLibrary.Concat_StrStr` (`KismetSystemLibrary.GetDisplayName` self) " was killed by [" (`KismetSystemLibrary.GetDisplayName` KilledBy) "].") false)
      (`self.EffectOnDeath` KilledBy)
      (`self.K2_DestroyActor`))))

(fn `Effect`
  (params (ActorThatProducedDamage :type "Actor Object Reference")))

(fn `EffectOnDeath`
  (params (Actor :type "Actor Object Reference")))

(fn `UserConstructionScript`)