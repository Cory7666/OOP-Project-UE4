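; BP_HHedgehog is a hittable, destroyable hedgehog that costs the player points when killed.
; It overrides EffectOnDeath to subtract 50 from the Score of the passed actor if that actor is a FirstPersonCharacter, then runs the parent's death effect.
; All other behavior comes from the parent class, as its remaining events only call the parent or are disabled.
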(event `self.ReceiveBeginPlay`
  (`parent.ReceiveBeginPlay`))

(fn `EffectOnDeath`
  (params (Actor :type "Actor Object Reference"))
  (bind _asfirst_person_character (cast `/Game/FirstPersonBP/Blueprints/FirstPersonCharacter` Actor)
    (:`then`
      (set `/Game/FirstPersonBP/Blueprints/FirstPersonCharacter.Score` (+ (`/Game/FirstPersonBP/Blueprints/FirstPersonCharacter.Score` _asfirst_person_character) -50) _asfirst_person_character))
    (:`CastFailed`
      _))
  (`parent.EffectOnDeath` Actor))

(fn `UserConstructionScript`
  (`parent.UserConstructionScript`))