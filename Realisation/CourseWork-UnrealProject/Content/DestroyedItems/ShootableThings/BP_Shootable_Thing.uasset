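; BP_Shootable_Thing is a moving actor that can be shot, damaged and killed, and has a set lifespan.
; Each tick it teleports along its forward vector by Speed scaled by delta time, keeping its rotation.
; TakeDamage responds only to one damage type, calling OnGetDamage, then OnDeath with the damager once Health is zero or below.
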(event `self.ReceiveBeginPlay`
  (`parent.ReceiveBeginPlay`)
  (set `self.LifeSpan` (`self.LifeSpan`)))

(event `self.ReceiveTick`
  (params (DeltaSeconds :type "Float (single-precision)"))
  (bind _defaultsceneroot (`self.DefaultSceneRoot`))
  (`self.K2_TeleportTo` (+ (* (`self.GetActorForwardVector`) (* DeltaSeconds (`self.Speed`))) (`SceneComponent.K2_GetComponentLocation` _defaultsceneroot)) (`SceneComponent.K2_GetComponentRotation` _defaultsceneroot))
  (`parent.ReceiveTick` DeltaSeconds))

(event `/Game/DestroyedItems/BPI_Damageable.Take Damage`
  (params (Damage :type "Float (single-precision)") (DamagedBy :type "Actor Object Reference") (DamageType :type "/Game/DestroyedItems/EDamage_Types Enum" :default "NewEnumerator0"))
  ;[1 1 1] On being fired
  (if (`|EnumEquality` DamageType "NewEnumerator0")
    (`self.OnGetDamage` Damage DamagedBy)
    (if (<= (`self.Health`) 0.0)
      (`self.OnDeath` DamagedBy))))

(fn `UserConstructionScript`
  (`parent.UserConstructionScript`))